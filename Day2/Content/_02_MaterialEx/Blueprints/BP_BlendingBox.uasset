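; BP_BlendingBox is an actor that animates a blend between cat and dog weights on its mesh material.
; On BeginPlay it creates a dynamic instance of the blend material, assigns it to the mesh, and waits a short random delay before starting.
; A timeline then drives the CatWeight and DogWeight scalar parameters as complementary values, so one rises as the other falls.
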(event `self.ReceiveBeginPlay`
  (bind _returnvalue (`PrimitiveComponent.CreateDynamicMaterialInstance` (`self.StaticMesh`) 0 "/Game/_02_MaterialEx/Materials/Mat_Blend.Mat_Blend" "None"))
  (bind _output_get (set `self.MatBlend` _returnvalue))
  (`PrimitiveComponent.SetMaterial` (`self.StaticMesh`) 0 _output_get)
  (`KismetSystemLibrary.Delay` (`KismetMathLibrary.RandomFloatInRange` 0.0 3.0))
  (`self.블렌딩시작`))

(event `블렌딩시작`
  (bind (_direction _blendingratio) (`Timeline|BlendingTexture`)
    (:`Update`
      (if (`KismetSystemLibrary.IsValid` (`self.MatBlend`))
        (`MaterialInstanceDynamic.SetScalarParameterValue` (`self.MatBlend`) "CatWeight" _blendingratio)
        (`MaterialInstanceDynamic.SetScalarParameterValue` (`self.MatBlend`) "DogWeight" (- 1.0 _blendingratio))))))

(fn `UserConstructionScript`)